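; Interactive door Blueprint operated by a button that the first-person player presses with the Interact input.
; Overlapping the interaction box enables input and opens a gate; leaving disables input and closes it.
; Each press plays a timeline-driven button animation macro, then a FlipFlop alternately plays or reverses the timeline that updates the door's relative location.
; The construction script places the button from a transform variable.
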(event `InputAction|Interact`
  (params (Key :type "Key Structure"))
  (:`Pressed`
    (`/Engine/EditorBlueprintResources/StandardMacros.Gate` true :!label _label
      (:`Exit`
        (bind (_direction _button_track) (`Timeline|Button Press` :!via `PlayFromStart`)
          (:`Update`
            (`SceneComponent.K2_SetRelativeLocation` (`self.button`) (`KismetMathLibrary.VLerp` (`self.Button Out`) (`self.Button In`) _button_track) false false))
          (:`Finished`
            (`/Engine/EditorBlueprintResources/StandardMacros.FlipFlop`
              (:`A`
                (bind (_direction_2 _door_track) (`Timeline|Door Timeline` :!label _label_2)
                  (:`Update`
                    (`SceneComponent.K2_SetRelativeLocation` (`self.Door`) (`self.New Location`) false false))))
              (:`B`
                (goto _label_2 :!via `Reverse`)))))))))

(event `self.interaction box.OnComponentBeginOverlap`
  (params (OverlappedComponent :type "PrimitiveComponent Object Reference") (OtherActor :type "Actor Object Reference") (OtherComp :type "PrimitiveComponent Object Reference") (OtherBodyIndex :type Integer) (bFromSweep :type Boolean) (SweepResult :type "HitResult Structure (by ref)"))
  (cast `/Game/Assets/Blueprints/FirstPersonCharacter` OtherActor)
  (`self.EnableInput` (`GameplayStatics.GetPlayerController` 0))
  (goto _label :!via `Open`))

(event `self.interaction box.OnComponentEndOverlap`
  (params (OverlappedComponent :type "PrimitiveComponent Object Reference") (OtherActor :type "Actor Object Reference") (OtherComp :type "PrimitiveComponent Object Reference") (OtherBodyIndex :type Integer))
  (cast `/Game/Assets/Blueprints/FirstPersonCharacter` OtherActor)
  (`self.DisableInput` (`GameplayStatics.GetPlayerController` 0))
  (goto _label :!via `Close`))

(fn `UserConstructionScript`
  (`SceneComponent.K2_SetRelativeTransform` (`self.button`) (`self.Button Transform`) false false))